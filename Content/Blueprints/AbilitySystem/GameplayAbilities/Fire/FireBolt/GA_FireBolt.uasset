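; GA_FireBolt is the Fire Bolt gameplay ability, which casts a projectile toward the point under the mouse cursor.
; On valid target data it stores the hit location, turns the caster to face it through CombatInterface and starts the cast montage.
; The Event.Montage.FireBolt gameplay event triggers SpawnProjectile at that location, and the ability ends after a short delay.
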(event `self.K2_ActivateAbility`
  (bind (_asynctaskproxy _datahandle) (`TargetDeltaUnderMouse.CreateTargetDataUnderMouse`)
    (:`ValidData`
      (set `self.ProjectileTargetLocation` (`.Location` (`GameplayStatics.BreakHitResult` (`AbilitySystemBlueprintLibrary.GetHitResultFromTargetData` _datahandle))))
      (bind _ascombat_interface (cast `CombatInterface` (`self.GetAvatarActorFromActorInfo`)))
      (`CombatInterface.UpdateFacingTarget` _ascombat_interface (`self.ProjectileTargetLocation`))
      (`AbilityTask_PlayMontageAndWait.CreatePlayMontageAndWaitProxy` "None" "/Game/Assets/Character/Animatons/Abilities/AM_Cast_FireBolt_StaticPose.AM_Cast_FireBolt_StaticPose"
        (:`then`
          (`AbilityTask_WaitGameplayEvent.WaitGameplayEvent` (struct :`TagName` "Event.Montage.FireBolt") null
            (:`EventReceived`
              (`self.SpawnProjectile` (`self.ProjectileTargetLocation`))
              (`KismetSystemLibrary.Delay` 0.5)
              (`self.K2_EndAbility`))))))))